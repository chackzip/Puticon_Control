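; Player controller that lets the player switch control between a human character and a robo character found in the level.
; A FlipFlop on the switch input repossesses the other pawn and swaps Enhanced Input mapping contexts.
; In robo mode, the view moves to a separate camera actor placed at the human's camera socket, and the human mesh is hidden.
; Move, look and attack inputs are forwarded to whichever character is current.
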(event Input|EnhancedActionEvents|EnhancedInputActionIA_Switch
  (params (ActionValue :type Boolean) (ElapsedSeconds :type Float%20%28double-precision%29) (TriggeredSeconds :type Float%20%28double-precision%29) (InputAction :type Input%20Action%20Object%20Reference :default "/Game/Control/BP/Input/IA_Switch.IA_Switch"))
  (bind _returnvalue (PlayerController|LocalPlayerSubsystems|GetEnhancedInputLocalPlayerSubsystem))
  (bind _returnvalue_2 (PlayerController|LocalPlayerSubsystems|GetEnhancedInputLocalPlayerSubsystem))
  (bind _robocameraactor (Variables|Default|GetRoboCameraActor))
  (bind _personcharacter (Variables|Default|GetPersonCharacter))
  (bind _robocharacter (Variables|Default|GetRoboCharacter))
  (:Triggered
    (Utilities|FlowControl|FlipFlop
      (:A
        (Pawn|UnPossess)
        (Pawn|Possess _robocharacter)
        (Variables|Default|SetCurrentControlCharacter _robocharacter)
        (Input|AddMappingContext _returnvalue "/Game/Control/BP/Input/IMC_RoboControl.IMC_RoboControl" 0 "(bIgnoreAllPressedKeysUntilRelease=True,bForceImmediately=False)")
        (Input|RemoveMappingContext _returnvalue "/Game/Control/BP/Input/IMC_Control.IMC_Control" "(bIgnoreAllPressedKeysUntilRelease=True,bForceImmediately=False)")
        (Default|SetCameraPos _robocameraactor (Transformation|GetSocketLocation (Variables|/Script/Engine.Character|GetMesh (Variables|Default|GetPersonCharacter)) "camera"))
        (Game|Player|SetViewTargetwithBlend _robocameraactor 0.0 "VTBlend_Linear" 0.0 false)
        (Rendering|SetVisibility (Variables|/Script/Engine.Character|GetMesh (Variables|Default|GetPersonCharacter)) false false))
      (:B
        (Pawn|UnPossess)
        (Pawn|Possess _personcharacter)
        (Variables|Default|SetCurrentControlCharacter _personcharacter)
        (Input|AddMappingContext _returnvalue_2 "/Game/Control/BP/Input/IMC_Control.IMC_Control" 0 "(bIgnoreAllPressedKeysUntilRelease=True,bForceImmediately=False)")
        (Input|RemoveMappingContext _returnvalue_2 "/Game/Control/BP/Input/IMC_RoboControl.IMC_RoboControl" "(bIgnoreAllPressedKeysUntilRelease=True,bForceImmediately=False)")
        (Game|Player|SetViewTargetwithBlend (Variables|Default|GetPersonCharacter) 0.0 "VTBlend_Linear" 0.0 false)
        (Rendering|SetVisibility (Variables|/Script/Engine.Character|GetMesh (Variables|Default|GetPersonCharacter)) true false)))))

(event Input|EnhancedActionEvents|EnhancedInputActionIA_Move
  (params (ActionValue :type Vector%202D%20Structure) (ElapsedSeconds :type Float%20%28double-precision%29) (TriggeredSeconds :type Float%20%28double-precision%29) (InputAction :type Input%20Action%20Object%20Reference :default "/Game/Control/BP/Input/IA_Move.IA_Move"))
  (:Triggered
    (Class|ControlCharacter|Move (Variables|Default|GetCurrentControlCharacter) ActionValue :!label _label))
  (:Completed
    (goto _label)))

(event Input|EnhancedActionEvents|EnhancedInputActionIA_Attack
  (params (ActionValue :type Vector%202D%20Structure) (ElapsedSeconds :type Float%20%28double-precision%29) (TriggeredSeconds :type Float%20%28double-precision%29) (InputAction :type Input%20Action%20Object%20Reference :default "/Game/Control/BP/Input/IA_Attack.IA_Attack"))
  (:Triggered
    (Class|ControlCharacter|Attack (Variables|Default|GetCurrentControlCharacter))))

(event Input|EnhancedActionEvents|EnhancedInputActionIA_Look
  (params (ActionValue :type Vector%202D%20Structure) (ElapsedSeconds :type Float%20%28double-precision%29) (TriggeredSeconds :type Float%20%28double-precision%29) (InputAction :type Input%20Action%20Object%20Reference :default "/Game/Control/BP/Input/IA_Look.IA_Look"))
  (:Triggered
    (Class|ControlCharacter|Look (Variables|Default|GetCurrentControlCharacter) ActionValue)))

(event EventBeginPlay
  (Input|AddMappingContext (PlayerController|LocalPlayerSubsystems|GetEnhancedInputLocalPlayerSubsystem) "/Game/Control/BP/Input/IMC_Control.IMC_Control" 0 "(bIgnoreAllPressedKeysUntilRelease=True,bForceImmediately=False)")
  (bind _ascontrol_character (Utilities|Casting|CastToControlCharacter (Game|GetPlayerCharacter 0)))
  (bind _output_get (Variables|Default|SetPersonCharacter _ascontrol_character))
  (Variables|Default|SetCurrentControlCharacter _output_get)
  (bind _returnvalue (Actor|GetActorOfClass "/Game/Control/BP/Chara/Player/BP_ControlRoboCharacter.BP_ControlRoboCharacter_C"))
  (Variables|Default|SetRoboCharacter _returnvalue)
  (bind _returnvalue_2 (Actor|GetActorOfClass "/Game/Control/BP/Chara/BP_ControlRoboCameraActor.BP_ControlRoboCameraActor_C"))
  (bind _output_get_2 (Variables|Default|SetRoboCameraActor _returnvalue_2))
  (Default|Initialize _output_get_2 (Variables|Default|GetRoboCharacter)))

(event EventTick
  (params (DeltaSeconds :type Float%20%28single-precision%29)))

(fn ConstructionScript)