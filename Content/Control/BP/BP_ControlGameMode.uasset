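; BP_ControlGameMode is the game mode that starts a match and handles its victory or defeat.
; BeginPlay shows the HUD, then initializes every BP_ControlRoboCharacter, playing the background music inside that loop, once per character.
; OnEnd stops the BGM reference, which this graph never assigns, shows the win or lose widget with its sound, and opens the title level after a delay.
; The GameEnd function is an empty stub.
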(event Custom|OnEnd
  (params (bVictory :type Boolean))
  (bind _returnvalue (Game|GetPlayerController 0))
  (Audio|Components|Audio|Stop (Variables|Default|GetBGM))
  (if bVictory
    (bind _returnvalue_2 (UserInterface|CreateWidget "/Game/Control/BP/UI/WBP_Victory.WBP_Victory_C" _returnvalue))
    (UserInterface|Viewport|AddtoViewport _returnvalue_2 0)
    (Audio|PlaySound2D "/Game/Control/Audio/SC_Vitory.SC_Vitory" 1.0 1.0 0.0 0 0 false)
    (else
      (bind _returnvalue_3 (UserInterface|CreateWidget "/Game/Control/BP/UI/WBP_Lose.WBP_Lose_C" _returnvalue))
      (UserInterface|Viewport|AddtoViewport _returnvalue_3 0)
      (Audio|PlaySound2D "/Game/Control/Audio/SC_Lose.SC_Lose" 1.0 1.0 0.0 0 0 false)))
  (Utilities|FlowControl|Delay 8.0)
  (Game|OpenLevel(byObjectReference) "/Game/Control/Level/TitleLevel.TitleLevel"))

(event EventBeginPlay
  (bind _returnvalue (UserInterface|CreateWidget "/Game/Control/BP/UI/WBP_HUD.WBP_HUD_C" (Game|GetPlayerController 0)))
  (UserInterface|Viewport|AddtoViewport _returnvalue 0)
  (bind _outactors (Actor|GetAllActorsOfClass "/Game/Control/BP/Chara/Player/BP_ControlRoboCharacter.BP_ControlRoboCharacter_C"))
  (for _array_element _outactors
    (Default|Initialize _array_element)
    (Audio|PlaySound2D "/Game/Control/Audio/SC_BGM.SC_BGM" 1.0 1.0 0.0 0 0 false)))

(event EventTick
  (params (DeltaSeconds :type Float%20%28single-precision%29)))

(fn ConstructionScript)

(fn GameEnd
  (params (bVictory :type Boolean))
  (if bVictory
    _))