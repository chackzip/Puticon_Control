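; Base destructible building that holds its Chaos geometry collection in place until it takes damage, then collapses.
; SetField applies a dynamic-state physics field culled to the Box component, setting pieces inside it static on BeginPlay.
; The first damage switches them to dynamic, waits a zero-length delay, pushes item 0 away from the damage causer and plays a 2D collapse sound.
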(event EventBeginPlay
  (CallFunction|SetField "Chaos_Object_Static"))

(event Game|Damage|EventAnyDamage
  (params (Damage :type Float%20%28single-precision%29) (DamageType :type Damage%20Type%20Object%20Reference) (InstigatedBy :type Controller%20Object%20Reference) (DamageCauser :type Actor%20Object%20Reference))
  (if (not (Variables|Default|GetbBreak))
    (Variables|Default|SetbBreak true)
    (CallFunction|SetField "Chaos_Object_Dynamic")
    (Utilities|FlowControl|Delay 0.0)
    (Class|GeometryCollectionComponent|ApplyLinearVelocity (Variables|Default|GetGeometryCollection) 0 (* (Math|Vector|Normalize (- (Transformation|GetActorLocation) (Transformation|GetActorLocation DamageCauser))) (Math|Conversions|ToVector(Float) 2e+03)))
    (Audio|PlaySound2D "/Game/StarterContent/Audio/Collapse_Cue.Collapse_Cue" 1.0 1.0 0.0 0 0 false)))

(fn ConstructionScript)

(fn SetField
  (params (State :type EObjectStateTypeEnum%20Enum :default "Chaos_NONE"))
  (Class|GeometryCollectionComponent|ApplyPhysicsField (Variables|Default|GetGeometryCollection) true "Chaos_DynamicState" 0 (Field|SetCullingField (Variables|Default|GetCullingField) (Field|SetBoxFalloff (Variables|Default|GetBoxFalloff) 1.0 0.0 1.0 0.0 (Transformation|GetWorldTransform (Variables|Default|GetBox)) "Field_Falloff_Linear") (Field|SetUniformInteger (Variables|Default|GetUniformInteger) (Math|Conversions|ToInteger(Byte) State)) "Field_Culling_Inside")))