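; BP_AttackCollision is a short-lived box hitbox that delivers attack hits, configured by an AttackData struct.
; On BeginPlay, Init sets the box's collision profile and size, draws a debug box and sets the lifespan from that data.
; Overlaps apply damage, spawn a hit effect and shake player 0's camera.
; Blow attacks also send BlowMessage with the attacker's location to a ControlCharacter target and use a separate shake.
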(event OnComponentBeginOverlap(Box)
  (params (OverlappedComponent :type Primitive%20Component%20Object%20Reference) (OtherActor :type Actor%20Object%20Reference) (OtherComp :type Primitive%20Component%20Object%20Reference) (OtherBodyIndex :type Integer) (bFromSweep :type Boolean) (SweepResult :type Hit%20Result%20Structure%20%28by%20ref%29))
  (bind _attack_data (Variables|Default|GetAttack%20Data))
  (Game|Damage|ApplyDamage OtherActor (.damage _attack_data) 0 (.owner _attack_data))
  (Effects|SpawnEmitteratLocation (.hiteffect _attack_data) (Transformation|GetActorLocation) "0, 0, 0" "2.000000,2.000000,2.000000")
  (if (.bblow _attack_data)
    (bind _ascontrol_character (Utilities|Casting|CastToControlCharacter OtherActor))
    (Class|BPICharacter|Blow(Message) _ascontrol_character (Transformation|GetActorLocation (.owner _attack_data)))
    (Game|Feedback|ClientStartCameraShake (Game|GetPlayerController 0) "/Game/Control/BP/Chara/Common/BP_CameraShake_Blow.BP_CameraShake_Blow_C" 1.0 "CameraLocal" "0, 0, 0")
    (else
      (Game|Feedback|ClientStartCameraShake (Game|GetPlayerController 0) "/Game/Control/BP/Chara/Common/BP_CameraShake_Normal.BP_CameraShake_Normal_C" 1.0 "CameraLocal" "0, 0, 0"))))

(event EventBeginPlay
  (CallFunction|Init (Variables|Default|GetAttack%20Data)))

(fn ConstructionScript)

(fn Init
  (params (AttackData :type ST%20Attack%20Data%20Structure))
  (bind _output_get (Variables|Default|SetAttack%20Data AttackData))
  (Collision|SetCollisionProfileName (Variables|Default|GetBox) (.collisionprofilename _output_get) true :!class /Script/Engine.PrimitiveComponent)
  (Components|Box|SetBoxExtent (Variables|Default|GetBox) (.size _output_get) true)
  (Rendering|Debug|DrawDebugBox :Center (Transformation|GetActorLocation) :Extent (.size (Variables|Default|GetAttack%20Data)) :Duration (.duration (Variables|Default|GetAttack%20Data)))
  (Actor|SetLifeSpan (.duration (Variables|Default|GetAttack%20Data))))