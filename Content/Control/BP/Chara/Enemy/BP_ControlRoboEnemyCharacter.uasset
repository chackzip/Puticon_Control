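; Enemy robot character for the Control game, built as a child Blueprint that supplies enemy-specific HP display, attack collision and death handling.
; It fills the HUD enemy HP gauge on BeginPlay, updates it through UpdateHpGauge and returns the EnemyAttack collision profile.
; On death it disables capsule collision, stops AI logic, hides itself behind a scaled explosion and calls OnEnd(true) on BP_ControlGameMode.
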(event EventBeginPlay
  (|CallParentFunction)
  (Default|SetEnemyHP (Default|GetHpGaige (Variables|Default|GetHUDWidget)) 1.0))

(event Collision|EventActorBeginOverlap
  (params (OtherActor :type Actor%20Object%20Reference)))

(event EventTick
  (params (DeltaSeconds :type Float%20%28single-precision%29)))

(fn ConstructionScript)

(fn UpdateHpGauge
  (params (Value :type Float%20%28double-precision%29))
  (Default|SetEnemyHP (Default|GetHpGaige (Variables|Default|GetHUDWidget)) Value))

(fn GetAttackCollisionProfileName
  (return "EnemyAttack"))

(fn Dead
  (Collision|SetCollisionEnabled (Variables|Default|GetCapsuleComponent) "NoCollision")
  (AI|Logic|StopLogic (Variables|/Script/AIModule.AIController|GetBrainComponent (AI|GetAIController self)) "")
  (Development|SetHiddeninGame (Variables|Default|GetCapsuleComponent) true true)
  (Effects|SpawnEmitteratLocation "/Game/StarterContent/Particles/P_Explosion.P_Explosion" (Transformation|GetActorLocation) "0, 0, 0" "4.000000,4.000000,4.000000")
  (bind _asbp_control_game_mode (Utilities|Casting|CastToBP_ControlGameMode (Game|GetGameMode)))
  (Default|OnEnd _asbp_control_game_mode true))