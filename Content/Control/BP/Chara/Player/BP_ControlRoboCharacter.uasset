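; Player-controlled robot character Blueprint that handles ability-driven attacks, damage and knockback.
; BeginPlay grants its ability list to the Ability System and caches the WBP_HUD widget; Attack then activates abilities by gameplay tag.
; AnyDamage lowers HP, updates the HUD gauge and calls Dead at zero, though Dead is still empty.
; Blow launches the character away from a given position with upward lift.
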(event EventBeginPlay
  (CallFunction|InitAbility)
  (bind _foundwidgets (Widget|GetAllWidgetsOfClass "/Game/Control/BP/UI/WBP_HUD.WBP_HUD_C" true))
  (Variables|Default|SetHUDWidget (Utilities|Array|Get(acopy) _foundwidgets))
  (Default|SetPlayerHP (Default|GetHpGaige (Variables|Default|GetHUDWidget)) 1.0))

(event EventBlow
  (params (BlowStartPos :type Vector :default "0, 0, 0"))
  (bind _returnvalue (Transformation|GetActorLocation))
  (bind _returnvalue_2 (Math|Conversions|ToVector(Float) 2.5e+03))
  (bind _returnvalue_3 (- _returnvalue BlowStartPos))
  (bind _returnvalue_4 (Math|Vector|Normalize _returnvalue_3))
  (bind _returnvalue_5 (* _returnvalue_4 _returnvalue_2))
  (Character|LaunchCharacter (Math|Vector|MakeVector (.x _returnvalue_5) (.y _returnvalue_5) 1e+03) false false))

(event EventTick
  (params (DeltaSeconds :type Float%20%28single-precision%29)))

(event EventAttack
  (Abilities|TryActivateAbilitiesbyTag (Variables|Default|GetAbilitySystem) (GameplayTags|MakeLiteralGameplayTagContainer "(GameplayTags=((TagName=\"Ability.Action.Attack\")))") true))

(event Game|Damage|EventAnyDamage
  (params (Damage :type Float%20%28single-precision%29) (DamageType :type Damage%20Type%20Object%20Reference) (InstigatedBy :type Controller%20Object%20Reference) (DamageCauser :type Actor%20Object%20Reference))
  (if (not (CallFunction|IsDead))
    (bind _output_get (Variables|Default|SetHP (Math|Float|Max(Float) (- (Variables|Default|GetHP) Damage) 0.0)))
    (CallFunction|UpdateHpGauge (/ _output_get (Variables|Default|GetMaxHP)))
    (if (<= (Variables|Default|GetHP) 0.0)
      (CallFunction|Dead))))

(fn ConstructionScript)

(fn InitAbility
  (for _array_element (Variables|Default|GetAbilities)
    (GameplayAbilities|GiveAbility (Variables|Default|GetAbilitySystem) _array_element 0 -1)))

(fn UpdateHpGauge
  (params (Value :type Float%20%28double-precision%29))
  (Default|SetPlayerHP (Default|GetHpGaige (Variables|Default|GetHUDWidget)) Value))

(fn GetAttackCollisionProfileName
  (return "PlayerAttack"))

(fn Dead)

(fn IsDead
  (return (<= (Variables|Default|GetHP) 0.0)))